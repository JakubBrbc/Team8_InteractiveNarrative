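; Quest component that tracks a five-item collection quest (chocolates, flowers, shovel, wine, watch), each item either found or bought.
; CreateQuest adds the WB_Quest checklist to the viewport, and each Found or Buy event ticks that item's check on the widget.
; Found events also notify the item's shopkeeper and hint NPCs, while Buy events notify the item's pickup actor.
; Targets are looked up by class on each call, assuming one instance each.
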(event `Create Quest`
  (bind _returnvalue (`|CreateWidget` "/Game/_Main/Blueprints/Widgets/WB_Quest.WB_Quest_C"))
  (bind _output_get (set `self.WBQuest` _returnvalue))
  (`UserWidget.AddToViewport` _output_get 0))

(event `FoundChocolates`
  (bind _foundwidgets (`WidgetBlueprintLibrary.GetAllWidgetsOfClass` "/Game/_Main/Blueprints/Widgets/WB_Quest.WB_Quest_C"))
  (`/Game/_Main/Blueprints/Widgets/WB_Quest.ChocolateCheck` (`|GetArrayItem` _foundwidgets))
  (bind _returnvalue (`GameplayStatics.GetActorOfClass` "/Game/_Main/Blueprints/NPC/NPC_ShopkeeperChocolate.NPC_ShopkeeperChocolate_C"))
  (`/Game/_Main/Blueprints/NPC/NPC_ShopkeeperChocolate.Is Collected Chocolate` _returnvalue)
  (bind _returnvalue_2 (`GameplayStatics.GetActorOfClass` "/Game/_Main/Blueprints/NPC/NPC_HintChocolate.NPC_HintChocolate_C"))
  (`/Game/_Main/Blueprints/NPC/NPC_HintChocolate.IsPickedUp` _returnvalue_2))

(event `BuyChocolates`
  (bind _foundwidgets (`WidgetBlueprintLibrary.GetAllWidgetsOfClass` "/Game/_Main/Blueprints/Widgets/WB_Quest.WB_Quest_C"))
  (`/Game/_Main/Blueprints/Widgets/WB_Quest.ChocolateCheck` (`|GetArrayItem` _foundwidgets))
  (bind _returnvalue (`GameplayStatics.GetActorOfClass` "/Game/_Main/Blueprints/Actors/BP_Chocolate.BP_Chocolate_C"))
  (`/Game/_Main/Blueprints/Actors/BP_Chocolate.Is Bought Chocolate` _returnvalue))

(event `FoundFlowers`
  (bind _foundwidgets (`WidgetBlueprintLibrary.GetAllWidgetsOfClass` "/Game/_Main/Blueprints/Widgets/WB_Quest.WB_Quest_C"))
  (`/Game/_Main/Blueprints/Widgets/WB_Quest.FlowersCheck` (`|GetArrayItem` _foundwidgets))
  (bind _returnvalue (`GameplayStatics.GetActorOfClass` "/Game/_Main/Blueprints/NPC/NPC_ShopkeeperFlower.NPC_ShopkeeperFlower_C"))
  (`/Game/_Main/Blueprints/NPC/NPC_ShopkeeperFlower.IsCollectedFlowers` _returnvalue)
  (bind _returnvalue_2 (`GameplayStatics.GetActorOfClass` "/Game/_Main/Blueprints/NPC/NPC_HintFlowers.NPC_HintFlowers_C"))
  (`/Game/_Main/Blueprints/NPC/NPC_HintFlowers.IsPickedUp` _returnvalue_2))

(event `BuyFlowers`
  (bind _foundwidgets (`WidgetBlueprintLibrary.GetAllWidgetsOfClass` "/Game/_Main/Blueprints/Widgets/WB_Quest.WB_Quest_C"))
  (`/Game/_Main/Blueprints/Widgets/WB_Quest.FlowersCheck` (`|GetArrayItem` _foundwidgets))
  (bind _returnvalue (`GameplayStatics.GetActorOfClass` "/Game/_Main/Blueprints/Actors/BP_Flowers.BP_Flowers_C"))
  (`/Game/_Main/Blueprints/Actors/BP_Flowers.IsBoughtFlowers` _returnvalue))

(event `FoundShovel`
  (bind _foundwidgets (`WidgetBlueprintLibrary.GetAllWidgetsOfClass` "/Game/_Main/Blueprints/Widgets/WB_Quest.WB_Quest_C"))
  (`/Game/_Main/Blueprints/Widgets/WB_Quest.ShovelCheck` (`|GetArrayItem` _foundwidgets))
  (bind _returnvalue (`GameplayStatics.GetActorOfClass` "/Game/_Main/Blueprints/NPC/NPC_ShopkeeperShovel.NPC_ShopkeeperShovel_C"))
  (`/Game/_Main/Blueprints/NPC/NPC_ShopkeeperShovel.Is Collected Shovel` _returnvalue)
  (bind _returnvalue_2 (`GameplayStatics.GetActorOfClass` "/Game/_Main/Blueprints/NPC/NPC_HintShovel.NPC_HintShovel_C"))
  (`/Game/_Main/Blueprints/NPC/NPC_HintShovel.IsPickedUP` _returnvalue_2))

(event `BuyShovel`
  (bind _foundwidgets (`WidgetBlueprintLibrary.GetAllWidgetsOfClass` "/Game/_Main/Blueprints/Widgets/WB_Quest.WB_Quest_C"))
  (`/Game/_Main/Blueprints/Widgets/WB_Quest.ShovelCheck` (`|GetArrayItem` _foundwidgets))
  (bind _returnvalue (`GameplayStatics.GetActorOfClass` "/Game/_Main/Blueprints/Actors/BP_Shovel.BP_Shovel_C"))
  (`/Game/_Main/Blueprints/Actors/BP_Shovel.Is Bought Shovel` _returnvalue))

(event `FoundWine`
  (bind _foundwidgets (`WidgetBlueprintLibrary.GetAllWidgetsOfClass` "/Game/_Main/Blueprints/Widgets/WB_Quest.WB_Quest_C"))
  (`/Game/_Main/Blueprints/Widgets/WB_Quest.WineCheck` (`|GetArrayItem` _foundwidgets))
  (bind _returnvalue (`GameplayStatics.GetActorOfClass` "/Game/_Main/Blueprints/NPC/NPC_ShopkeeperWine.NPC_ShopkeeperWine_C"))
  (`/Game/_Main/Blueprints/NPC/NPC_ShopkeeperWine.Is Collected Wine` _returnvalue)
  (bind _returnvalue_2 (`GameplayStatics.GetActorOfClass` "/Game/_Main/Blueprints/NPC/NPC_HintWine.NPC_HintWine_C"))
  (`/Game/_Main/Blueprints/NPC/NPC_HintWine.IsPickedUp` _returnvalue_2))

(event `BuyWine`
  (bind _foundwidgets (`WidgetBlueprintLibrary.GetAllWidgetsOfClass` "/Game/_Main/Blueprints/Widgets/WB_Quest.WB_Quest_C"))
  (`/Game/_Main/Blueprints/Widgets/WB_Quest.WineCheck` (`|GetArrayItem` _foundwidgets))
  (bind _returnvalue (`GameplayStatics.GetActorOfClass` "/Game/_Main/Blueprints/Actors/BP_Wine.BP_Wine_C"))
  (`/Game/_Main/Blueprints/Actors/BP_Wine.Is Bought Wine` _returnvalue))

(event `FoundWatch`
  (bind _foundwidgets (`WidgetBlueprintLibrary.GetAllWidgetsOfClass` "/Game/_Main/Blueprints/Widgets/WB_Quest.WB_Quest_C"))
  (`/Game/_Main/Blueprints/Widgets/WB_Quest.WatchCheck` (`|GetArrayItem` _foundwidgets))
  (bind _returnvalue (`GameplayStatics.GetActorOfClass` "/Game/_Main/Blueprints/NPC/NPC_ShopkeeperWatch.NPC_ShopkeeperWatch_C"))
  (`/Game/_Main/Blueprints/NPC/NPC_ShopkeeperWatch.Is Collected Watch` _returnvalue)
  (bind _returnvalue_2 (`GameplayStatics.GetActorOfClass` "/Game/_Main/Blueprints/NPC/NPC_HintWatch.NPC_HintWatch_C"))
  (`/Game/_Main/Blueprints/NPC/NPC_HintWatch.IsPickedUp` _returnvalue_2))

(event `BuyWatch`
  (bind _foundwidgets (`WidgetBlueprintLibrary.GetAllWidgetsOfClass` "/Game/_Main/Blueprints/Widgets/WB_Quest.WB_Quest_C"))
  (`/Game/_Main/Blueprints/Widgets/WB_Quest.WatchCheck` (`|GetArrayItem` _foundwidgets))
  (bind _returnvalue (`GameplayStatics.GetActorOfClass` "/Game/_Main/Blueprints/Actors/BP_Watch.BP_Watch_C"))
  (`/Game/_Main/Blueprints/Actors/BP_Watch.Is Bought Watch` _returnvalue))