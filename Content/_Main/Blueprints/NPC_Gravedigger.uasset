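; NPC_Gravedigger is an NPC Blueprint that steps through a dialogue array each time its Talk event fires.
; It creates a WB_DialogBox widget when none is valid, writes the current line into it, and disables player movement during the conversation.
; With an existing widget, index 5 skips the text update.
; Once the lines run out, it restores walking and removes the widget.
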(event `/Game/_Main/Blueprints/BPI_Dialog.Talk`
  (bind _charactermovement (`Character.CharacterMovement` (`GameplayStatics.GetPlayerCharacter` 0)))
  (`/Engine/EditorBlueprintResources/StandardMacros.IncrementInt` (`self.TalkIndex`)
    (:`  `
      (if (< (`self.TalkIndex`) (`KismetArrayLibrary.Array_Length` (`self.Dialogue`)))
        (`CharacterMovementComponent.DisableMovement` _charactermovement)
        (`self.UI`
          (:`then`
            (if (not (== (`self.TalkIndex`) 5))
              (`TextBlock.SetText` (`/Game/_Main/Blueprints/WB_DialogBox.DialogueText_NPC` (`self.UI`)) (`KismetTextLibrary.Conv_StringToText` (`|GetArrayItem` (`self.Dialogue`) (`self.TalkIndex`))) :!label _label)))
          (:`else`
            (bind _returnvalue (`|CreateWidget` "/Game/_Main/Blueprints/WB_DialogBox.WB_DialogBox_C" (`GameplayStatics.GetPlayerController` 0)))
            (bind _output_get (set `self.UI` _returnvalue))
            (`UserWidget.AddToViewport` _output_get 0)
            (goto _label)))
        (else
          (`CharacterMovementComponent.SetMovementMode` _charactermovement "MOVE_Walking" 0)
          (`Widget.RemoveFromParent` (`self.UI`)))))))

(fn `UserConstructionScript`)