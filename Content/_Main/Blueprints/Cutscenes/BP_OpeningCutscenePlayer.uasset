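; BP_OpeningCutscenePlayer plays the opening cutscene video and starts the game when it ends.
; PlayOpeningcutscene creates WB_OpeningCutscene if needed, adds it to the viewport and opens the source on the media player.
; It then binds CloseVideo to the player's end-reached event.
; CloseVideo removes the widget and calls GameStart on BP_ThirdPersonGameMode, found through GetActorOfClass.
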(event `After its played`
  (add `MediaPlayer.OnEndReached` (`self.CutsceneMediaPlayer`) (delegate `CloseVideo`)))

(event `CloseVideo`
  (`Widget.RemoveFromParent` (`self.CutsceneWidget`))
  (bind _returnvalue (`GameplayStatics.GetActorOfClass` "/Game/ThirdPerson/Blueprints/BP_ThirdPersonGameMode.BP_ThirdPersonGameMode_C"))
  (`/Game/ThirdPerson/Blueprints/BP_ThirdPersonGameMode.Game start` _returnvalue))

(event `PlayOpening cutscene`
  (`self.CutsceneWidget`
    (:`then`
      _)
    (:`else`
      (bind _returnvalue (`|CreateWidget` "/Game/_Main/Blueprints/Cutscenes/WB_OpeningCutscene.WB_OpeningCutscene_C" (`GameplayStatics.GetPlayerController` 0)))
      (bind _output_get (set `self.CutsceneWidget` _returnvalue))))
  (`UserWidget.AddToViewport` _output_get 0)
  (`MediaPlayer.OpenSource` (`self.CutsceneMediaPlayer`) "/Game/_Main/Blueprints/Cutscenes/Opening_Cutscene.Opening_Cutscene")
  (`self.After its played`))

(fn `UserConstructionScript`)