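; BP_EndingCutscenePlayer plays the good or bad ending video cutscene.
; Each play event creates or reuses its own WB_OpeningCutscene widget, adds it to the viewport and opens the matching source on the shared CutsceneMediaPlayer.
; It then binds the player's end-reached event to a handler that removes that widget from the screen.
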(event `TrackEndingGood`
  (add `MediaPlayer.OnEndReached` (`self.CutsceneMediaPlayer`) (delegate `CloseCutscene`)))

(event `CloseCutscene`
  (`Widget.RemoveFromParent` (`self.CutsceneWidget2`)))

(event `TrackEndingBad`
  (add `MediaPlayer.OnEndReached` (`self.CutsceneMediaPlayer`) (delegate `CloseVideo`)))

(event `CloseVideo`
  (`Widget.RemoveFromParent` (`self.CutsceneWidget`)))

(event `PlayBadEnding`
  (`self.CutsceneWidget`
    (:`then`
      _)
    (:`else`
      (bind _returnvalue (`|CreateWidget` "/Game/_Main/Blueprints/Cutscenes/WB_OpeningCutscene.WB_OpeningCutscene_C" (`GameplayStatics.GetPlayerController` 0)))
      (bind _output_get (set `self.CutsceneWidget` _returnvalue))))
  (`UserWidget.AddToViewport` _output_get 0)
  (`MediaPlayer.OpenSource` (`self.CutsceneMediaPlayer`) "/Game/_Main/Blueprints/Cutscenes/Bad_ending_.Bad_ending_")
  (`self.TrackEndingBad`))

(event `PlayGoodEnding`
  (`self.CutsceneWidget2`
    (:`then`
      _)
    (:`else`
      (bind _returnvalue (`|CreateWidget` "/Game/_Main/Blueprints/Cutscenes/WB_OpeningCutscene.WB_OpeningCutscene_C" (`GameplayStatics.GetPlayerController` 0)))
      (bind _output_get (set `self.CutsceneWidget2` _returnvalue))))
  (`UserWidget.AddToViewport` _output_get 0)
  (`MediaPlayer.OpenSource` (`self.CutsceneMediaPlayer`) "/Game/_Main/Blueprints/Cutscenes/good_ending.good_ending")
  (`self.TrackEndingGood`))

(fn `UserConstructionScript`)