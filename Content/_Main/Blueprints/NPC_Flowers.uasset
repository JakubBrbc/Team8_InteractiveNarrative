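; NPC_Flowers is an NPC that plays a linear dialogue, shown in a WB_DialogBox widget.
; Each Talk call advances TalkIndex through the Dialogue array, disabling player movement, then restores walking and removes the widget after the last line.
; A TriggerZone overlap shows a TextRender to the third-person character while lines remain and hides it on exit.
; TalkIndex never resets here, so the conversation does not replay.
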(event `/Game/_Main/Blueprints/BPI_Dialog.Talk`
  (bind _charactermovement (`Character.CharacterMovement` (`GameplayStatics.GetPlayerCharacter` 0)))
  (`/Engine/EditorBlueprintResources/StandardMacros.IncrementInt` (`self.TalkIndex`)
    (:`  `
      (if (< (`self.TalkIndex`) (`KismetArrayLibrary.Array_Length` (`self.Dialogue`)))
        (`CharacterMovementComponent.DisableMovement` _charactermovement)
        (`self.UI`
          (:`then`
            _)
          (:`else`
            (bind _returnvalue (`|CreateWidget` "/Game/_Main/Blueprints/WB_DialogBox.WB_DialogBox_C" (`GameplayStatics.GetPlayerController` 0)))
            (bind _output_get (set `self.UI` _returnvalue))
            (`UserWidget.AddToViewport` _output_get 0)))
        (`TextBlock.SetText` (`/Game/_Main/Blueprints/WB_DialogBox.DialogueText_NPC` (`self.UI`)) (`KismetTextLibrary.Conv_StringToText` (`|GetArrayItem` (`self.Dialogue`) (`self.TalkIndex`))))
        (else
          (`CharacterMovementComponent.SetMovementMode` _charactermovement "MOVE_Walking" 0)
          (`Widget.RemoveFromParent` (`self.UI`)))))))

(event `self.Trigger Zone.OnComponentBeginOverlap`
  (params (OverlappedComponent :type "PrimitiveComponent Object Reference") (OtherActor :type "Actor Object Reference") (OtherComp :type "PrimitiveComponent Object Reference") (OtherBodyIndex :type Integer) (bFromSweep :type Boolean) (SweepResult :type "HitResult Structure (by ref)"))
  (cast `/Game/ThirdPerson/Blueprints/BP_ThirdPersonCharacter` OtherActor)
  (if (< (`self.TalkIndex`) (`KismetArrayLibrary.Array_Length` (`self.Dialogue`)))
    (`SceneComponent.SetHiddenInGame` (`self.TextRender`) false false)))

(event `self.Trigger Zone.OnComponentEndOverlap`
  (params (OverlappedComponent :type "PrimitiveComponent Object Reference") (OtherActor :type "Actor Object Reference") (OtherComp :type "PrimitiveComponent Object Reference") (OtherBodyIndex :type Integer))
  (cast `/Game/ThirdPerson/Blueprints/BP_ThirdPersonCharacter` OtherActor)
  (`SceneComponent.SetHiddenInGame` (`self.TextRender`) true false))

(fn `UserConstructionScript`)