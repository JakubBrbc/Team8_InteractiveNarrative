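; NPC Blueprint that turns into a zombie when infected and awards currency.
; The Infect event hides the normal Mesh and reveals the Zombie component in its place.
; It then adds a fixed amount to the Blueprint's own Currency variable and writes the total to a WB_Curency widget.
; The widget is created and added to the viewport on demand if this instance has no valid one.
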(event `/Game/_Main/Blueprints/BPI_Infect.Infect`
  (`SceneComponent.SetHiddenInGame` (`self.Mesh`) true false)
  (`SceneComponent.SetHiddenInGame` (`self.Zombie`) false false)
  (`self.UI_Currency`
    (:`then`
      _)
    (:`else`
      (bind _returnvalue (`|CreateWidget` "/Game/_Main/Blueprints/WB_Curency.WB_Curency_C"))
      (bind _output_get (set `self.UI_Currency` _returnvalue))
      (`UserWidget.AddToViewport` _output_get 0)))
  (set `self.Currency` (+ (`self.Currency`) 25))
  (`TextBlock.SetText` (`/Game/_Main/Blueprints/WB_Curency.TextBlock_0` (`self.UI_Currency`)) (`KismetTextLibrary.Conv_IntToText` (`self.Currency`))))

(fn `UserConstructionScript`)