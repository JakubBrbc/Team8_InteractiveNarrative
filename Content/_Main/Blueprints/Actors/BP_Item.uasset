(event `Is already collected`)

(event `/Game/_Main/Blueprints/Interface/BPI_Dialog.Talk`
  (bind _charactermovement (`Character.CharacterMovement` (`GameplayStatics.GetPlayerCharacter` 0)))
  (bind _result (`/Engine/EditorBlueprintResources/StandardMacros.IncrementInt` (`self.EPress`))
    (:`  `
      (`SceneComponent.SetHiddenInGame` (`self.Chocolate`) true false)
      (if (< _result 2)
        (`CharacterMovementComponent.DisableMovement` _charactermovement)
        (bind _returnvalue (`|CreateWidget` "/Game/_Main/Blueprints/Widgets/WB_YouGotItem.WB_YouGotItem_C"))
        (bind _output_get (set `self.UI` _returnvalue))
        (`UserWidget.AddToViewport` _output_get 0)
        (`SceneComponent.SetHiddenInGame` (`self.TextRender`) true false)
        (else
          (`CharacterMovementComponent.SetMovementMode` _charactermovement "MOVE_Walking" 0)
          (`Widget.RemoveFromParent` (`self.UI`))
          (`/Game/_Main/Blueprints/AC_Quest.FoundChocolates` (`self.AC_Quest`)))))))

(event `self.Sphere.OnComponentBeginOverlap`
  (params (OverlappedComponent :type "PrimitiveComponent Object Reference") (OtherActor :type "Actor Object Reference") (OtherComp :type "PrimitiveComponent Object Reference") (OtherBodyIndex :type Integer) (bFromSweep :type Boolean) (SweepResult :type "HitResult Structure (by ref)"))
  (cast `/Game/ThirdPerson/Blueprints/BP_ThirdPersonCharacter` OtherActor)
  (if (< (`self.EPress`) 2)
    (`SceneComponent.SetHiddenInGame` (`self.TextRender`) false false)))

(event `self.Sphere.OnComponentEndOverlap`
  (params (OverlappedComponent :type "PrimitiveComponent Object Reference") (OtherActor :type "Actor Object Reference") (OtherComp :type "PrimitiveComponent Object Reference") (OtherBodyIndex :type Integer))
  (cast `/Game/ThirdPerson/Blueprints/BP_ThirdPersonCharacter` OtherActor)
  (`SceneComponent.SetHiddenInGame` (`self.TextRender`) true false))

(fn `UserConstructionScript`)