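; BP_InfectionsHint is a trigger actor that shows a one-time infections hint when the player character enters its box.
; The first overlap by a BP_ThirdPersonCharacter disables movement and look input, shows the mouse cursor and displays the WB_InfectionsHint widget.
; A CloseHint event restores walking, look input and the hidden cursor, then removes the widget.
; The DoOnce precedes the character cast, so any overlapping actor can consume the trigger.
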(event `self.Box.OnComponentBeginOverlap`
  (params (OverlappedComponent :type "PrimitiveComponent Object Reference") (OtherActor :type "Actor Object Reference") (OtherComp :type "PrimitiveComponent Object Reference") (OtherBodyIndex :type Integer) (bFromSweep :type Boolean) (SweepResult :type "HitResult Structure (by ref)"))
  (bind _returnvalue (`GameplayStatics.GetPlayerController` 0))
  (`/Engine/EditorBlueprintResources/StandardMacros.DoOnce` false
    (:`Completed`
      (cast `/Game/ThirdPerson/Blueprints/BP_ThirdPersonCharacter` OtherActor)
      (`CharacterMovementComponent.DisableMovement` (`Character.CharacterMovement` (`GameplayStatics.GetPlayerCharacter` 0)))
      (bind _output_get (set `PlayerController.bShowMouseCursor` true _returnvalue))
      (`Controller.SetIgnoreLookInput` _returnvalue _output_get)
      (bind _returnvalue_2 (`|CreateWidget` "/Game/_Main/Blueprints/Widgets/WB_InfectionsHint.WB_InfectionsHint_C"))
      (`UserWidget.AddToViewport` _returnvalue_2 0))))

(event `CloseHint`
  (bind _returnvalue (`GameplayStatics.GetPlayerController` 0))
  (`CharacterMovementComponent.SetMovementMode` (`Character.CharacterMovement` (`GameplayStatics.GetPlayerCharacter` 0)) "MOVE_Walking" 0)
  (bind _output_get (set `PlayerController.bShowMouseCursor` false _returnvalue))
  (`Controller.SetIgnoreLookInput` _returnvalue _output_get)
  (`Widget.RemoveFromParent` (stale `self.Box.OnComponentBeginOverlap` _returnvalue_2)))

(fn `UserConstructionScript`)