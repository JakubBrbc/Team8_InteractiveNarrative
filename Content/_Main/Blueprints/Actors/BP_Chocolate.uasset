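; Collectible chocolate actor that the player picks up through the Talk event to progress a quest.
; A press counter drives two stages: pickup hides the mesh, freezes movement and shows an item widget with sound, then the next press closes it, restores walking and notifies ACQuest.
; Sphere overlap toggles the hint text for uncollected chocolate.
; IsBoughtChocolate sets the counter to its collected state, blocking further pickup.
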(event `Is Bought Chocolate`
  ;[1 1 1] Setting value for item already collected
  (set `self.EPress` 3))

(event `/Game/_Main/Blueprints/Interface/BPI_Dialog.Talk`
  (bind _charactermovement (`Character.CharacterMovement` (`GameplayStatics.GetPlayerCharacter` 0)))
  ;[1 1 1] Cecking if Item was collected
  (if (< (`self.EPress`) 3)
    ;[1 1 1] Setting value of E presses
    (bind _result (`/Engine/EditorBlueprintResources/StandardMacros.IncrementInt` (`self.EPress`))
      (:`  `
        ;[1 1 1] Hidding item in game after collection
        (`SceneComponent.SetHiddenInGame` (`self.Chocolate`) true false)
        (if (< _result 2)
          ;[1 1 1] Disabling movement becouse player in widget
          (`CharacterMovementComponent.DisableMovement` _charactermovement)
          ;[1 1 1] Creating You got item widget
          (bind _returnvalue (`|CreateWidget` "/Game/_Main/Blueprints/Widgets/WB_YouGotItem.WB_YouGotItem_C"))
          (bind _output_get (set `self.UI` _returnvalue))
          (`UserWidget.AddToViewport` _output_get 0)
          ;[1 1 1] Hiding E to collect hint
          (`SceneComponent.SetHiddenInGame` (`self.TextRender`) true false)
          ;[1 1 1] Once playing you got item sound
          (`/Engine/EditorBlueprintResources/StandardMacros.DoOnce` false
            (:`Completed`
              (`GameplayStatics.PlaySound2D` "/Engine/VREditor/Sounds/UI/Object_PickUp.Object_PickUp" 1.0 1.0 0.0 null null)))
          (else
            ;[1 1 1] Enabling movement
            (`CharacterMovementComponent.SetMovementMode` _charactermovement "MOVE_Walking" 0)
            ;[1 1 1] Removing widget from view
            (`Widget.RemoveFromParent` (`self.UI`))
            ;[1 1 1] Casting Event for BP Quest Component
            (`/Game/_Main/Blueprints/BP_QuestComponent.FoundChocolates` (`self.AC_Quest`))))))))

(event `self.Sphere.OnComponentBeginOverlap`
  (params (OverlappedComponent :type "PrimitiveComponent Object Reference") (OtherActor :type "Actor Object Reference") (OtherComp :type "PrimitiveComponent Object Reference") (OtherBodyIndex :type Integer) (bFromSweep :type Boolean) (SweepResult :type "HitResult Structure (by ref)"))
  ;[1 1 1] When Player in collision sphere display hint text and only displeing when item not collected
  (cast `/Game/ThirdPerson/Blueprints/BP_ThirdPersonCharacter` OtherActor)
  (if (< (`self.EPress`) 2)
    (`SceneComponent.SetHiddenInGame` (`self.TextRender`) false false)))

(event `self.Sphere.OnComponentEndOverlap`
  (params (OverlappedComponent :type "PrimitiveComponent Object Reference") (OtherActor :type "Actor Object Reference") (OtherComp :type "PrimitiveComponent Object Reference") (OtherBodyIndex :type Integer))
  ;[1 1 1] When player leves collision sphere hide hint text
  (cast `/Game/ThirdPerson/Blueprints/BP_ThirdPersonCharacter` OtherActor)
  (`SceneComponent.SetHiddenInGame` (`self.TextRender`) true false))

(fn `UserConstructionScript`)