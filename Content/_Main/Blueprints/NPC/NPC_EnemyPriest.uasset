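; Enemy priest NPC that wanders around its starting location and chases the player on sight.
; Roam and FollowPlayer loop through AI MoveTo calls, re-checking the SeeingPlayer flag whenever a move succeeds or fails.
; PawnSensing sightings of the third-person character set the flag and start the chase.
; A retriggerable SearchTime delay clears it and resumes roaming once sightings stop, with debug prints marking both switches.
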(event `self.ReceiveBeginPlay`
  (set `self.Random Location` (`self.K2_GetActorLocation`))
  (`self.Roam`))

(event `Roam`
  (if (`self.Seeing Player`)
    (`self.FollowPlayer`)
    (else
      (`|AIMoveTo` self (`NavigationSystemV1.K2_GetRandomReachablePointInRadius` (`self.Random Location`) 2000.0 null null) null
        (:`then`
          (if (`self.Seeing Player`)
            (`self.FollowPlayer`)))
        (:`OnSuccess`
          (if (`self.Seeing Player`) :!label _label
            (`self.FollowPlayer`)
            (else
              (`self.Roam`))))
        (:`OnFail`
          (goto _label))))))

(event `FollowPlayer`
  (`|AIMoveTo` self (0.0 0.0 0.0) (`self.Player Followed`)
    (:`OnSuccess`
      _)
    (:`OnFail`
      _))
  (if (`self.Seeing Player`)
    (`self.FollowPlayer`)
    (else
      (`self.Roam`))))

(event `self.PawnSensing.OnSeePawn`
  (params (Pawn :type "Pawn Object Reference"))
  (bind _asbp_third_person_character (cast `/Game/ThirdPerson/Blueprints/BP_ThirdPersonCharacter` Pawn))
  (set `self.Player Followed` _asbp_third_person_character)
  (`|ExecutionSequence`
    (:`then_0`
      (set `self.Seeing Player` true)
      (`KismetSystemLibrary.PrintString` "Hello")
      (`self.FollowPlayer`))
    (:`then_1`
      (`KismetSystemLibrary.RetriggerableDelay` (`self.Search Time`))
      (set `self.Seeing Player` false)
      (`KismetSystemLibrary.PrintString` "Roam")
      (`self.Roam`))))

(fn `UserConstructionScript`)