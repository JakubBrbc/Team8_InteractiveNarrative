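; Shopkeeper NPC that sells a watch tied to a quest, showing a hint text while the player is in its trigger sphere and the watch is uncollected.
; Talk opens the WB_Shopkeeper dialogue widget, locking movement and look input until Leave or a successful Buy.
; Buy checks the game mode's Currency, then either calls BuyWatch on the quest component or plays an insufficient-funds animation.
; IsCollectedWatch sets IsBought, disabling further talk and hints.
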(event `/Game/_Main/Blueprints/Interface/BPI_Dialog.Talk`
  (bind _returnvalue (`GameplayStatics.GetPlayerController` 0))
  ;[1 1 1] Checking if item has been colected or bought
  (if (== (`self.IsBought`) 0)
    ;[1 1 1] Disabeling movement for player becouse player in widget
    (`CharacterMovementComponent.DisableMovement` (`Character.CharacterMovement` (`GameplayStatics.GetPlayerCharacter` 0)))
    ;[1 1 1] Showing mouse cursor in game and disabling option to move camera
    (bind _output_get (set `PlayerController.bShowMouseCursor` true _returnvalue))
    (`Controller.SetIgnoreLookInput` _returnvalue _output_get)
    ;[1 1 1] Creating Shop Widget
    (bind _returnvalue_2 (`|CreateWidget` "/Game/_Main/Blueprints/Widgets/WB_Shopkeeper.WB_Shopkeeper_C"))
    (bind _output_get_2 (set `self.UI` _returnvalue_2))
    (`UserWidget.AddToViewport` _output_get_2 0)
    ;[1 1 1] Setting dialogue for shopkeeper
    (`TextBlock.SetText` (`/Game/_Main/Blueprints/Widgets/WB_Shopkeeper.DialogueText_NPC` (`self.UI`)) (`KismetTextLibrary.Conv_StringToText` (`self.Dialogue`)))))

(event `Leave`
  (bind _returnvalue (`GameplayStatics.GetPlayerController` 0))
  ;[1 1 1] After pressing leave enabeling movement for player, removing widget, hidding mouse cursor and enabling camera movement
  (`CharacterMovementComponent.SetMovementMode` (`Character.CharacterMovement` (`GameplayStatics.GetPlayerCharacter` 0)) "MOVE_Walking" 0)
  (`Widget.RemoveFromParent` (`self.UI`))
  (bind _output_get (set `PlayerController.bShowMouseCursor` false _returnvalue))
  (`Controller.SetIgnoreLookInput` _returnvalue _output_get))

(event `Buy`
  (bind _returnvalue (`GameplayStatics.GetPlayerController` 0))
  (bind _ui (`self.UI`))
  ;[1 1 1] After pressing buy checking if player has enought money
  (bind _returnvalue_2 (`GameplayStatics.GetActorOfClass` "/Game/ThirdPerson/Blueprints/BP_ThirdPersonGameMode.BP_ThirdPersonGameMode_C"))
  (if (>= (`/Game/ThirdPerson/Blueprints/BP_ThirdPersonGameMode.Currency` _returnvalue_2) 50)
    ;[1 1 1] Completing Quest in BP_QuestComponent
    (`/Game/_Main/Blueprints/BP_QuestComponent.BuyWatch` (`self.AC_Quest`))
    ;[1 1 1] After Buying item enabeling movement for player, removing widget, hidding mouse cursor and enabling camera movement
    (`Widget.RemoveFromParent` (`self.UI`))
    (`CharacterMovementComponent.SetMovementMode` (`Character.CharacterMovement` (`GameplayStatics.GetPlayerCharacter` 0)) "MOVE_Walking" 0)
    (bind _output_get (set `PlayerController.bShowMouseCursor` false _returnvalue))
    (`Controller.SetIgnoreLookInput` _returnvalue _output_get)
    (else
      ;[1 1 1] If player doesn't have enought money displaying insufficient funds animation in widget
      (`Widget.SetVisibility` (`/Game/_Main/Blueprints/Widgets/WB_Shopkeeper.Insufficientfunds` (`self.UI`)) "Visible")
      (`UserWidget.PlayAnimation` _ui (`/Game/_Main/Blueprints/Widgets/WB_Shopkeeper.Insufficient_Anim` _ui) 0.0 1 "Forward" 1.0 false))))

(event `Is Collected Watch`
  ;[1 1 1] Setting value for ittem alredy has been colected
  (set `self.IsBought` 2))

(event `self.Trigger.OnComponentBeginOverlap`
  (params (OverlappedComponent :type "PrimitiveComponent Object Reference") (OtherActor :type "Actor Object Reference") (OtherComp :type "PrimitiveComponent Object Reference") (OtherBodyIndex :type Integer) (bFromSweep :type Boolean) (SweepResult :type "HitResult Structure (by ref)"))
  ;[1 1 1] When Player in collision sphere display hint text and only displeing when item not collected
  (cast `/Game/ThirdPerson/Blueprints/BP_ThirdPersonCharacter` OtherActor)
  (if (== (`self.IsBought`) 0)
    (`SceneComponent.SetHiddenInGame` (`self.TextRender`) false false)))

(event `self.Trigger.OnComponentEndOverlap`
  (params (OverlappedComponent :type "PrimitiveComponent Object Reference") (OtherActor :type "Actor Object Reference") (OtherComp :type "PrimitiveComponent Object Reference") (OtherBodyIndex :type Integer))
  ;[1 1 1] When player leves collision sphere hide hint text
  (cast `/Game/ThirdPerson/Blueprints/BP_ThirdPersonCharacter` OtherActor)
  (`SceneComponent.SetHiddenInGame` (`self.TextRender`) true false))

(fn `UserConstructionScript`)