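; Gravedigger NPC that plays a scripted two-speaker dialogue, starts a quest and later reports the game ending.
; Each Talk call advances the line index, locks player movement and shows the line as David or John in the dialogue widget, created on first use.
; After the last line, a FlipFlop alternates between a one-time movement restore with quest creation and printing a good or bad ending from the game mode's infection count.
; A trigger zone toggles a text prompt.
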(event `/Game/_Main/Blueprints/Interface/BPI_Dialog.Talk`
  (bind _charactermovement (`Character.CharacterMovement` (`GameplayStatics.GetPlayerCharacter` 0)))
  (`/Engine/EditorBlueprintResources/StandardMacros.IncrementInt` (`self.TalkIndex`)
    (:`  `
      (if (< (`self.TalkIndex`) (`KismetArrayLibrary.Array_Length` (`self.Dialogue`)))
        (`CharacterMovementComponent.DisableMovement` _charactermovement)
        (`self.UI`
          (:`then`
            (switch `int` (`self.TalkIndex`)
              (:`0`
                (`TextBlock.SetText` (`/Game/_Main/Blueprints/Widgets/WB_DialogGraveKeeper.DialogueText_DAvid` (`self.UI`)) (`KismetTextLibrary.Conv_StringToText` (`|GetArrayItem` (`self.Dialogue`) (`self.TalkIndex`))) :!label _label)
                (`/Game/_Main/Blueprints/Widgets/WB_DialogGraveKeeper.VisibleDavid` (`self.UI`)))
              (:`1`
                (`TextBlock.SetText` (`/Game/_Main/Blueprints/Widgets/WB_DialogGraveKeeper.DialogueText_John` (`self.UI`)) (`KismetTextLibrary.Conv_StringToText` (`|GetArrayItem` (`self.Dialogue`) (`self.TalkIndex`))) :!label _label_2)
                (`/Game/_Main/Blueprints/Widgets/WB_DialogGraveKeeper.VisibleJohn` (`self.UI`)))
              (:`2`
                (goto _label))
              (:`3`
                (goto _label_2))
              (:`4`
                (goto _label))
              (:`5`
                (goto _label))
              (:`6`
                (goto _label_2))
              (:`7`
                (goto _label))
              (:`8`
                (goto _label_2))
              (:`9`
                (goto _label))
              (:`10`
                (goto _label_2))
              (:`11`
                (goto _label))
              (:`12`
                (goto _label))))
          (:`else`
            (bind _returnvalue (`|CreateWidget` "/Game/_Main/Blueprints/Widgets/WB_DialogGraveKeeper.WB_DialogGraveKeeper_C" (`GameplayStatics.GetPlayerController` 0)))
            (bind _output_get (set `self.UI` _returnvalue))
            (`UserWidget.AddToViewport` _output_get 0)
            (goto _label)))
        (else
          (`/Engine/EditorBlueprintResources/StandardMacros.FlipFlop`
            (:`A`
              (`/Engine/EditorBlueprintResources/StandardMacros.DoOnce` false
                (:`Completed`
                  (`CharacterMovementComponent.SetMovementMode` _charactermovement "MOVE_Walking" 0)
                  (`Widget.RemoveFromParent` (`self.UI`))
                  (set `PlayerController.bShowMouseCursor` false (`GameplayStatics.GetPlayerController` 0))
                  (`/Game/_Main/Blueprints/AC_Quest.Create Quest` (`self.AC_Quest`)))))
            (:`B`
              (bind _returnvalue_2 (`GameplayStatics.GetActorOfClass` "/Game/ThirdPerson/Blueprints/BP_ThirdPersonGameMode.BP_ThirdPersonGameMode_C"))
              (if (> (`/Game/ThirdPerson/Blueprints/BP_ThirdPersonGameMode.Infections` _returnvalue_2) 0)
                (`KismetSystemLibrary.PrintString` "Bad ending")
                (else
                  (`KismetSystemLibrary.PrintString` "Good ending"))))))))))

(event `self.Trigger Zone.OnComponentBeginOverlap`
  (params (OverlappedComponent :type "PrimitiveComponent Object Reference") (OtherActor :type "Actor Object Reference") (OtherComp :type "PrimitiveComponent Object Reference") (OtherBodyIndex :type Integer) (bFromSweep :type Boolean) (SweepResult :type "HitResult Structure (by ref)"))
  (cast `/Game/ThirdPerson/Blueprints/BP_ThirdPersonCharacter` OtherActor)
  (if (< (`self.TalkIndex`) (`KismetArrayLibrary.Array_Length` (`self.Dialogue`)))
    (`SceneComponent.SetHiddenInGame` (`self.TextRender`) false false)))

(event `self.Trigger Zone.OnComponentEndOverlap`
  (params (OverlappedComponent :type "PrimitiveComponent Object Reference") (OtherActor :type "Actor Object Reference") (OtherComp :type "PrimitiveComponent Object Reference") (OtherBodyIndex :type Integer))
  (cast `/Game/ThirdPerson/Blueprints/BP_ThirdPersonCharacter` OtherActor)
  (`SceneComponent.SetHiddenInGame` (`self.TextRender`) true false))

(fn `UserConstructionScript`)