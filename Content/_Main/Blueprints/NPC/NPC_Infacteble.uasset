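; Infectable NPC that turns into a zombie and awards currency through the third-person game mode.
; Infect looks up the game mode and compares a local counter to its Infections value, clamping it down when higher.
; Once they are equal, it hides the normal mesh, shows the Zombie component, plays a zombie sound, copies UICurrency and calls AddCurrency.
; The counter is never incremented in this graph.
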(event `/Game/_Main/Blueprints/Interface/BPI_Infect.Infect`
  (bind _infections (`/Game/ThirdPerson/Blueprints/BP_ThirdPersonGameMode.Infections` (`self.BP_Gamemode`)))
  (bind _returnvalue (`GameplayStatics.GetActorOfClass` "/Game/ThirdPerson/Blueprints/BP_ThirdPersonGameMode.BP_ThirdPersonGameMode_C"))
  (set `self.BP_Gamemode` _returnvalue)
  (if (not (< (`self.Variable`) (`/Game/ThirdPerson/Blueprints/BP_ThirdPersonGameMode.Infections` (`self.BP_Gamemode`))))
    (bind _output_get (set `self.Variable` _infections)))
  (if (== _output_get _infections)
    (`SceneComponent.SetHiddenInGame` (`self.Mesh`) true false)
    (`SceneComponent.SetHiddenInGame` (`self.Zombie`) false false)
    (`GameplayStatics.PlaySound2D` "/Game/_Main/Blueprints/Sound/270472__littlerobotsoundfactory__zombie_03_2.270472__littlerobotsoundfactory__zombie_03_2" 1.0 1.0 0.0 null null)
    (set `self.UI Currency` (`/Game/ThirdPerson/Blueprints/BP_ThirdPersonGameMode.UI_Currency` (`self.BP_Gamemode`)))
    (`/Game/ThirdPerson/Blueprints/BP_ThirdPersonGameMode.AddCurrency` (`self.BP_Gamemode`))))

(fn `UserConstructionScript`)