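; Shopkeeper NPC that shows a text prompt while the player character overlaps its trigger and opens a dialogue shop widget on Talk.
; Talk creates WB_Shopkeeper with the NPC's dialogue, disables movement and look input, and shows the cursor; Leave reverses this.
; Buy checks the game mode's Currency against a hardcoded price and only handles insufficient funds, showing an animated warning without completing purchases.
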(event `/Game/_Main/Blueprints/Interface/BPI_Dialog.Talk`
  (bind _returnvalue (`GameplayStatics.GetPlayerController` 0))
  (if true
    (`CharacterMovementComponent.DisableMovement` (`Character.CharacterMovement` (`GameplayStatics.GetPlayerCharacter` 0)))
    (bind _output_get (set `PlayerController.bShowMouseCursor` true _returnvalue))
    (`Controller.SetIgnoreLookInput` _returnvalue _output_get)
    (bind _returnvalue_2 (`|CreateWidget` "/Game/_Main/Blueprints/Widgets/WB_Shopkeeper.WB_Shopkeeper_C"))
    (bind _output_get_2 (set `self.UI` _returnvalue_2))
    (`UserWidget.AddToViewport` _output_get_2 0)
    (`TextBlock.SetText` (`/Game/_Main/Blueprints/Widgets/WB_Shopkeeper.DialogueText_NPC` (`self.UI`)) (`KismetTextLibrary.Conv_StringToText` (`self.Dialogue`)))))

(event `Leave`
  (bind _returnvalue (`GameplayStatics.GetPlayerController` 0))
  (`CharacterMovementComponent.SetMovementMode` (`Character.CharacterMovement` (`GameplayStatics.GetPlayerCharacter` 0)) "MOVE_Walking" 0)
  (`Widget.RemoveFromParent` (`self.UI`))
  (bind _output_get (set `PlayerController.bShowMouseCursor` false _returnvalue))
  (`Controller.SetIgnoreLookInput` _returnvalue _output_get))

(event `Buy`
  (bind _returnvalue (`GameplayStatics.GetActorOfClass` "/Game/ThirdPerson/Blueprints/BP_ThirdPersonGameMode.BP_ThirdPersonGameMode_C"))
  (if (not (>= (`/Game/ThirdPerson/Blueprints/BP_ThirdPersonGameMode.Currency` _returnvalue) 50))
    (`Widget.SetVisibility` (`/Game/_Main/Blueprints/Widgets/WB_Shopkeeper.Insufficientfunds` (`self.UI`)) "Visible")
    (`UserWidget.PlayAnimation` (`self.UI`) (`/Game/_Main/Blueprints/Widgets/WB_Shopkeeper.Insufficient_Anim` (`self.UI`)) 0.0 1 "Forward" 1.0 false)))

(event `self.Trigger.OnComponentBeginOverlap`
  (params (OverlappedComponent :type "PrimitiveComponent Object Reference") (OtherActor :type "Actor Object Reference") (OtherComp :type "PrimitiveComponent Object Reference") (OtherBodyIndex :type Integer) (bFromSweep :type Boolean) (SweepResult :type "HitResult Structure (by ref)"))
  (cast `/Game/ThirdPerson/Blueprints/BP_ThirdPersonCharacter` OtherActor)
  (if true
    (`SceneComponent.SetHiddenInGame` (`self.TextRender`) false false)))

(event `self.Trigger.OnComponentEndOverlap`
  (params (OverlappedComponent :type "PrimitiveComponent Object Reference") (OtherActor :type "Actor Object Reference") (OtherComp :type "PrimitiveComponent Object Reference") (OtherBodyIndex :type Integer))
  (cast `/Game/ThirdPerson/Blueprints/BP_ThirdPersonCharacter` OtherActor)
  (`SceneComponent.SetHiddenInGame` (`self.TextRender`) true false))

(fn `UserConstructionScript`)